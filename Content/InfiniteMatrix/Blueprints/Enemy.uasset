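; Enemy actor that drifts toward the player's Y and Z position while holding its own X, destroying itself once its X falls below the player's.
; Construction randomizes its scale, health and a Speed value that the movement does not use.
; Projectile hits decrement health, and a kill increments the shooter's score and destroys both actors.
; Touching the player deals damage, clears the owning tunnel's IncrementScore flag and destroys the enemy.
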(event OnComponentBeginOverlap(Sphere)
  (params (OverlappedComponent :type Primitive%20Component%20Object%20Reference) (OtherActor :type Actor%20Object%20Reference) (OtherComp :type Primitive%20Component%20Object%20Reference) (OtherBodyIndex :type Integer) (bFromSweep :type Boolean) (SweepResult :type Hit%20Result%20Structure%20%28by%20ref%29))
  (bind _asprojectile (Utilities|Casting|CastToProjectile OtherActor)
    (:then
      (bind _isdead (CallFunction|DecHealth))
      (if _isdead
        (Default|IncScore (Variables|/Game/InfiniteMatrix/Blueprints/Projectile.Projectile_C|GetPlayer _asprojectile))
        (Actor|DestroyActor _asprojectile)
        (Actor|DestroyActor :!label _label)))
    (:CastFailed
      (bind _asbp_player (Utilities|Casting|CastToBP_Player OtherActor))
      (Default|TakeDamage _asbp_player 0.3)
      (Variables|/Game/InfiniteMatrix/Blueprints/BP_Tunnel.BP_Tunnel_C|SetIncrementScore (Variables|Default|GetOwningTunnel self) false)
      (goto _label))))

(event EventTick
  (params (DeltaSeconds :type Float%20%28single-precision%29))
  (bind _returnvalue (Game|Player|GetPlayerPawn 0))
  (bind _returnvalue_2 (Transformation|GetActorLocation))
  (bind _returnvalue_3 (Transformation|GetActorLocation _returnvalue))
  (if (< (.x _returnvalue_2) (.x _returnvalue_3))
    (Actor|DestroyActor)
    (else
      (Transformation|SetActorLocation (Math|Interpolation|VInterpTo (Math|Vector|MakeVector (.x _returnvalue_2) (.y _returnvalue_2) (.z _returnvalue_2)) (Math|Vector|MakeVector (.x _returnvalue_2) (.y _returnvalue_3) (.z _returnvalue_3)) DeltaSeconds 2.0) false false))))

(fn ConstructionScript
  (bind _returnvalue (Math|Random|RandomFloatinRange 1.0 3.0))
  (Transformation|SetActorScale3D (* (Transformation|GetActorScale3D) _returnvalue))
  (Variables|Default|SetSpeed (/ 3.0 _returnvalue))
  (Variables|Default|SetHealth (Math|Float|Truncate _returnvalue)))

(fn DecHealth
  (bind _result (Math|Integer|DecrementInt (Variables|Default|GetHealth))
    (:%20%20
      (Variables|Default|SetHealth _result)
      (return (<= _result 0)))))